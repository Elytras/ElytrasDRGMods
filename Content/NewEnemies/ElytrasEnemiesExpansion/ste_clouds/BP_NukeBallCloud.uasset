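; BP_NukeBallCloud is a cloud actor Blueprint from an enemy expansion that builds on its parent class's behavior.
; On BeginPlay it runs the parent logic and binds to its own OnDestroyed event.
; When destroyed, it sets the Enabled parameter on the NSFieldBorderIceOpr effect to zero, switching off that field border effect.
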(event `self.ReceiveBeginPlay`
  (`parent.ReceiveBeginPlay`)
  (add `Actor.OnDestroyed` (delegate `Destroyed`)))

(event `Destroyed`
  (params (DestroyedActor :type "Actor Object Reference"))
  (`FXSystemComponent.SetIntParameter` (`self.NS_FieldBorder_Ice_Opr`) "Enabled" 0))

(fn `UserConstructionScript`
  (`parent.UserConstructionScript`))