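; BP_TeleportCloud is an enemy-expansion cloud actor, named for teleporting, with an electric Niagara field border effect.
; It defers setup to its parent class and binds a handler to its own destruction on BeginPlay.
; When destroyed, it sets the Niagara Enabled variable to zero to switch off the border effect.
; No teleport logic appears in this graph, and its overlap and Tick events are unused.
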(event `Destroyed`
  (params (DestroyedActor :type "Actor Object Reference"))
  (`NiagaraComponent.SetVariableInt` (`self.NS_FieldBorder_Electric`) "Enabled" 0))

(event `self.ReceiveBeginPlay`
  (`parent.ReceiveBeginPlay`)
  (add `Actor.OnDestroyed` (delegate `Destroyed`)))

(fn `UserConstructionScript`
  (`parent.UserConstructionScript`))