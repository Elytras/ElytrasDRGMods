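; BP_FireCloud is a temporary fire cloud hazard with Niagara fire and a burning sound, using a status effect trigger component.
; On spawn it scales the sound attenuation and audio trigger sphere from the main sphere's radius and starts a lifetime timer.
; The local player entering the audio sphere fades the looping sound in.
; When the lifetime expires, it disables the fire effect and fades the sound out.
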(event `self.ReceiveBeginPlay`
  (bind _sphereradius (`SphereComponent.SphereRadius` (`self.Sphere`)))
  (bind _returnvalue (* _sphereradius 1.5))
  (`parent.ReceiveBeginPlay`)
  (set `StatusEffectTriggerComponent.collider` null (`self.StatusEffectTrigger`))
  (`ActorComponent.SetTickGroup` (`self.NS_Fire`) "TG_PostUpdateWork")
  (`KismetSystemLibrary.K2_SetTimerDelegate` (delegate `Timer`) (`self.Lifetime`))
  (bind _outattenuationsettings (`AudioComponent.BP_GetAttenuationSettingsToApply` (`self.Burning`)))
  (bind _structout (setmembers `SoundAttenuationSettings` :`StructRef` _outattenuationsettings :`AttenuationShapeExtents` (`KismetMathLibrary.MakeVector` (/ _sphereradius 4.0)) :`FalloffDistance` _returnvalue))
  (set `AudioComponent.AttenuationOverrides` _structout (`self.Burning`))
  (`SphereComponent.SetSphereRadius` (`self.AudioSphere`) _returnvalue true)
  (`AudioComponent.SetBoolParameter` (`self.Burning`) "Looping" true))

(event `Timer`
  (set `self.Stopped` true)
  (`FXSystemComponent.SetIntParameter` (`self.NS_Fire`) "Enabled" 0)
  (`AudioComponent.FadeOut` (`self.Burning`) 1.0 0.0 "Logarithmic"))

(event `self.AudioSphere.OnComponentBeginOverlap`
  (params (OverlappedComponent :type "PrimitiveComponent Object Reference") (OtherActor :type "Actor Object Reference") (OtherComp :type "PrimitiveComponent Object Reference") (OtherBodyIndex :type Integer) (bFromSweep :type Boolean) (SweepResult :type "HitResult Structure (by ref)"))
  (if (and (== (`GameFunctionLibrary.GetLocalPlayerCharacter`) OtherActor) (not (`self.Stopped`)))
    (`AudioComponent.FadeIn` (`self.Burning`) 1.0 1.75 0.0 "Logarithmic")))

(fn `UserConstructionScript`
  (`parent.UserConstructionScript`))