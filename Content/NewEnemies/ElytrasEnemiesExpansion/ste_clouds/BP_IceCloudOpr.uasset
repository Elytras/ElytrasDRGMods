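; BP_IceCloudOpr is an ice cloud actor that shows a Niagara border effect and plays a freezing sound for a limited lifetime.
; On BeginPlay it scales the sound's attenuation and an audio trigger sphere from the main Sphere radius.
; The player entering the trigger starts the sound, which replays whenever it finishes.
; When the Lifetime timer expires, it sets Stopped, disables the effect and fades out the audio without destroying the actor.
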(event `self.ReceiveBeginPlay`
  (bind _sphereradius (`SphereComponent.SphereRadius` (`self.Sphere`)))
  (bind _returnvalue (* _sphereradius 1.5))
  (`parent.ReceiveBeginPlay`)
  (`KismetSystemLibrary.K2_SetTimerDelegate` (delegate `Timer`) (`self.Lifetime`))
  (bind _outattenuationsettings (`AudioComponent.BP_GetAttenuationSettingsToApply` (`self.Freezing`)))
  (bind _structout (setmembers `SoundAttenuationSettings` :`StructRef` _outattenuationsettings :`AttenuationShapeExtents` (`KismetMathLibrary.MakeVector` (/ _sphereradius 4.0)) :`FalloffDistance` _returnvalue))
  (set `AudioComponent.AttenuationOverrides` _structout (`self.Freezing`))
  (`SphereComponent.SetSphereRadius` (`self.AudioSphere`) _returnvalue true))

(event `Timer`
  (set `self.Stopped` true)
  (`FXSystemComponent.SetIntParameter` (`self.NS_FieldBorder_Ice_Opr`) "Enabled" 0)
  (`AudioComponent.FadeOut` (`self.Freezing`) 2.0 0.0 "Logarithmic"))

(event `self.AudioSphere.OnComponentBeginOverlap`
  (params (OverlappedComponent :type "PrimitiveComponent Object Reference") (OtherActor :type "Actor Object Reference") (OtherComp :type "PrimitiveComponent Object Reference") (OtherBodyIndex :type Integer) (bFromSweep :type Boolean) (SweepResult :type "HitResult Structure (by ref)"))
  (if (and (`KismetMathLibrary.ClassIsChildOf` (`GameplayStatics.GetObjectClass` OtherActor) "/Game/Character/BP_PlayerCharacter.BP_PlayerCharacter_C") (not (`self.Stopped`)))
    (`AudioComponent.Play` (`self.Freezing`) 0.0)))

(event `self.Freezing.OnAudioFinished`
  (if (not (`self.Stopped`))
    (`AudioComponent.Play` (`self.Freezing`) 0.0)))

(fn `UserConstructionScript`
  (`parent.UserConstructionScript`))