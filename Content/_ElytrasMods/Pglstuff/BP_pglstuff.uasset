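; Mod actor that lets the local player trigger the effects of live grenade launcher projectiles on all players with either thumb mouse button.
; On BeginPlay it waits for a valid local character and controller, then enables input on itself.
; Each press loops every PRJ_GrenadeLauncher against every player character, calling the projectile's LaunchPlayer and DamageArmorClients and adding a randomly directed impulse to the player.
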(event `self.ReceiveBeginPlay`
  (bind _returnvalue (`GameFunctionLibrary.GetLocalPlayerCharacter`))
  (bind _returnvalue_2 (`PlayerCharacter.GetPlayerController` _returnvalue))
  (`/Game/_ElytrasMods/ModManager/Libraries/EMM_ActorMacros.WaitForValid` _returnvalue
    (:`Is Valid`
      (`/Game/_ElytrasMods/ModManager/Libraries/EMM_ActorMacros.WaitForValid` _returnvalue_2
        (:`Is Valid`
          (`self.EnableInput` _returnvalue_2))))))

(event `Key|ThumbMouseButton` :consume false
  (params (Key :type "Key Structure"))
  (:`Pressed`
    (bind _outactors (`GameplayStatics.GetAllActorsOfClass` "/Game/WeaponsNTools/GrenadeLauncher/PRJ_GrenadeLauncher.PRJ_GrenadeLauncher_C" :!label _label))
    (for _array_element _outactors
      (for _array_element_2 (`ActorFunctionLibrary.GetAllPlayerCharacters`)
        (`/Game/WeaponsNTools/GrenadeLauncher/PRJ_GrenadeLauncher.LaunchPlayer` _array_element _array_element_2)
        (`PlayerCharacter.AddImpulseFromVector` _array_element_2 (* (`KismetMathLibrary.RandomUnitVector`) 1000.0))
        (`ExplosionBaseComponent.DamageArmorClients` _array_element (`GameplayStatics.MakeHitResult` false) (`/Game/WeaponsNTools/GrenadeLauncher/PRJ_GrenadeLauncher.Damage` _array_element))))))

(event `Key|ThumbMouseButton2` :consume false
  (params (Key :type "Key Structure"))
  (:`Pressed`
    (goto _label)))

(fn `UserConstructionScript`)